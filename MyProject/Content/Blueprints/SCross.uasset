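; SCross is an interactable cross that the player can bless.
; A box overlap shows an interaction prompt widget, created at BeginPlay, while the cross is unblessed and removes it when the player leaves.
; The Interact event increments the first-person character's Blessmade counter, makes the static mesh visible, removes the prompt and sets IsBlessed, which only suppresses later prompts without guarding against repeated interaction.
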(event OnComponentEndOverlap(Box)
  (params (OverlappedComponent :type Primitive%20Component%20Object%20Reference) (OtherActor :type Actor%20Object%20Reference) (OtherComp :type Primitive%20Component%20Object%20Reference) (OtherBodyIndex :type Integer))
  ;[1 1 1] Prompt
  (if (== (Game|GetPlayerCharacter 0) OtherActor)
    (Widget|RemovefromParent (Variables|Default|GetInteractpromt))))

(event OnComponentBeginOverlap(Box)
  (params (OverlappedComponent :type Primitive%20Component%20Object%20Reference) (OtherActor :type Actor%20Object%20Reference) (OtherComp :type Primitive%20Component%20Object%20Reference) (OtherBodyIndex :type Integer) (bFromSweep :type Boolean) (SweepResult :type Hit%20Result%20Structure%20%28by%20ref%29))
  ;[1 1 1] Prompt
  (if (== OtherActor (Game|GetPlayerCharacter 0))
    (if (not (Variables|Default|GetisBlessed))
      (UserInterface|Viewport|AddtoViewport (Variables|Default|GetInteractpromt) 0))))

(event EventBeginPlay
  (bind _returnvalue (UserInterface|CreateWidget "/Game/W_interactionprompt.W_interactionprompt_C"))
  (Variables|Default|SetInteractpromt _returnvalue))

(event EventInteract
  ;[1 1 1] bless
  (bind _asbp_first_person_character (Utilities|Casting|CastToBP_FirstPersonCharacter (Game|GetPlayerCharacter 0)))
  (Variables|/Game/FirstPerson/Blueprints/BP_FirstPersonCharacter.BP_FirstPersonCharacter_C|SetBlessmade _asbp_first_person_character (+ (Variables|/Game/FirstPerson/Blueprints/BP_FirstPersonCharacter.BP_FirstPersonCharacter_C|GetBlessmade _asbp_first_person_character) 1))
  (Rendering|SetVisibility (Variables|Components|GetStaticMesh) true false)
  (Widget|RemovefromParent (Variables|Default|GetInteractpromt))
  (Variables|Default|SetisBlessed true))

(fn ConstructionScript)