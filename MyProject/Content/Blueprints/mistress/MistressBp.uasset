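; Mistress AI character that spots the player through pawn sensing and reacts via a behavior tree.
; On BeginPlay its AI controller runs the Runnerbt behavior tree.
; When PawnSensing sees a pawn tagged Player, it sets the seeingplayer blackboard flag to true for the tree to use.
; This graph never clears that flag.
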(event OnSeePawn(PawnSensing)
  (params (Pawn :type Pawn%20Object%20Reference))
  (if (Actor|ActorHasTag Pawn "Player")
    (AI|Components|Blackboard|SetValueasBool (AI|GetBlackboard (AI|GetAIController self)) (Utilities|Name|MakeLiteralName "seeingplayer") true)))

(event EventBeginPlay
  (AI|RunBehaviorTree (AI|GetAIController self) "/Game/Blueprints/Runner/Runnerbt.Runnerbt"))

(fn ConstructionScript)