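; Walker enemy Blueprint for a horror game that chases the player on sight and ends the game with a jumpscare when it reaches them.
; PawnSensing sets a seeing flag and starts an AI MoveTo toward player 0; the flag is never cleared.
; On arrival, a one-time jumpscare disables input, blends the view to the walker and turns on its spotlight.
; After a delay it pauses the game and shows the Game_over widget with UI-only mouse input.
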(event OnSeePawn(PawnSensing)
  (params (Pawn :type Pawn%20Object%20Reference))
  (Variables|Default|Setisseeingplayer true)
  (CallFunction|ChasePlayer))

(event Custom|Chase%20player
  (bind _returnvalue (Game|GetPlayerCharacter 0))
  (bind _returnvalue_2 (Game|GetPlayerController 0))
  (bind _returnvalue_3 (Game|GetPlayerController 0))
  (if (Variables|Default|Getisseeingplayer)
    (AI|AIMoveTo self "0, 0, 0" _returnvalue 5.0 false
      (:OnSuccess
        (if (not (Variables|Default|GetJumpscared))
          (Input|DisableInput _returnvalue _returnvalue_3)
          (Game|Player|SetViewTargetwithBlend _returnvalue_3 self 0.0 "VTBlend_Linear" 0.0 false)
          (Rendering|SetVisibility (Variables|Default|GetSpotLight) true false)
          (Variables|Default|SetJumpscared true)
          (Utilities|FlowControl|Delay 3.0)
          (Game|SetGamePaused true)
          (bind _returnvalue_4 (UserInterface|CreateWidget "/Game/Game_over.Game_over_C"))
          (UserInterface|Viewport|AddtoViewport _returnvalue_4 0)
          (Variables|/Script/Engine.PlayerController|SetbShowMouseCursor _returnvalue_2 true)
          (Input|SetInputModeUIOnly _returnvalue_2 _returnvalue_4 "DoNotLock" false))))))

(fn ConstructionScript)